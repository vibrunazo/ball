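; HUD Blueprint that puts the ball character's health and a coin count on screen.
; On BeginPlay it creates the Ballhudwidget and adds it to the viewport.
; Each Tick it casts the owning pawn to ballchar and pushes the truncated Takedamagecomponent health to the P1 HP text, showing zero when the cast fails.
; A setcoins event passes coin values through to the widget.
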(event `set coins`
  (params (coins :type Integer))
  (`/Game/hud/ballhudwidget.set coins text` (`self.hudwidget`) coins))

(event `self.ReceiveBeginPlay`
  (bind _returnvalue (`|CreateWidget` "/Game/hud/ballhudwidget.ballhudwidget_C"))
  (bind _output_get (set `self.hudwidget` _returnvalue))
  (`UserWidget.AddToViewport` _output_get 0))

(event `self.ReceiveTick`
  (params (DeltaSeconds :type "Float (single-precision)"))
  (bind _asballchar (cast `/Game/bp/chars/ball/ballchar` (`self.GetOwningPawn`))
    (:`then`
      (`/Game/hud/ballhudwidget.Set p1hp text` (`self.hudwidget`) (`KismetMathLibrary.FTrunc` (`/Game/bp/takedamagecomponent.health` (`/Game/bp/chars/ball/ballchar.takedamagecomponent` _asballchar)))))
    (:`CastFailed`
      (`/Game/hud/ballhudwidget.Set p1hp text` (`self.hudwidget`) 0))))

(fn `UserConstructionScript`)